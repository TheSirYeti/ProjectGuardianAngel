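; Default player controller that routes Enhanced Input to the main character.
; On possess it caches the pawn as BP_MainCharacter, and on BeginPlay it adds the IMC_BaseCharacter mapping context.
; Movement and jump input actions are forwarded to the cached character's DoMovement, ExecuteJump and EndJump functions, leaving the behavior itself to the character.
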(event Input|EnhancedActionEvents|EnhancedInputActionIA_BaseMovement
  (params (ActionValue :type Vector%202D%20Structure) (ElapsedSeconds :type Float%20%28double-precision%29) (TriggeredSeconds :type Float%20%28double-precision%29) (InputAction :type Input%20Action%20Object%20Reference :default "/Game/Inputs/BaseCharacter/IA_BaseMovement.IA_BaseMovement"))
  (Default|DoMovement (Variables|Default|GetMainCharacter) ActionValue))

(event Input|EnhancedActionEvents|EnhancedInputActionIA_Jump
  (params (ActionValue :type Boolean) (ElapsedSeconds :type Float%20%28double-precision%29) (TriggeredSeconds :type Float%20%28double-precision%29) (InputAction :type Input%20Action%20Object%20Reference :default "/Game/Inputs/BaseCharacter/IA_Jump.IA_Jump"))
  (bind _maincharacter (Variables|Default|GetMainCharacter))
  (:Started
    (Default|ExecuteJump _maincharacter))
  (:Completed
    (Default|EndJump _maincharacter)))

(event EventPossess
  (params (PossessedPawn :type Pawn%20Object%20Reference))
  (bind _asbp_main_character (Utilities|Casting|CastToBP_MainCharacter PossessedPawn))
  (Variables|Default|SetMainCharacter _asbp_main_character))

(event EventBeginPlay
  (Input|AddMappingContext (PlayerController|LocalPlayerSubsystems|GetEnhancedInputLocalPlayerSubsystem) "/Game/Inputs/BaseCharacter/IMC_BaseCharacter.IMC_BaseCharacter" 0 "(bIgnoreAllPressedKeysUntilRelease=True,bForceImmediately=False,bNotifyUserSettings=False)"))

(fn ConstructionScript)