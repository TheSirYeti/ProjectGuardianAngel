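; BP_House is a procedural house actor that builds a floor and four walls from static mesh pieces in its Construction Script.
; Nested loops over Length and Width lay the floor grid at FloorSeparation spacing, then one loop per side places the walls, with side walls rotated.
; One wall branches on index modulo DoorCounter to add one of two components, likely alternating wall and door pieces.
; The event graph has no active logic.
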(event EventBeginPlay)

(event Collision|EventActorBeginOverlap
  (params (OtherActor :type Actor%20Object%20Reference)))

(event EventTick
  (params (DeltaSeconds :type Float%20%28single-precision%29)))

(fn ConstructionScript
  (bind _floorseparation (Variables|Measurements|GetFloorSeparation))
  (bind _baserotation (Variables|Default|GetBaseRotation))
  (bind _width (Variables|Dimensions|GetWidth))
  (bind _returnvalue (+ _baserotation 90))
  (bind _returnvalue_2 (* _width _floorseparation))
  (bind _returnvalue_3 (Math|Conversions|ToFloat(Integer) _returnvalue_2))
  (bind _returnvalue_4 (Math|Conversions|ToFloat(Integer) _returnvalue))
  ;[0.15 0.15 0.15 0.5] Piso
  (for _index (range 0 (- (Variables|Dimensions|GetLength) 1))
    (for _index_2 (range 0 (- (Variables|Dimensions|GetWidth) 1))
      (AddComponent|AddStaticMeshComponent false (Math|Transform|MakeTransform (Math|Vector|MakeVector (Math|Conversions|ToFloat(Integer) (* _index_2 (Variables|Measurements|GetFloorSeparation))) (Math|Conversions|ToFloat(Integer) (* _index (Variables|Measurements|GetFloorSeparation))) 0.0) (Math|Rotator|MakeRotator 0.0 0.0 0.0) "1.000000,1.000000,1.000000"))))
  ;[0.15 0.15 0.15 0.5] Pared 1
  (for _index_3 (range 0 (- (Variables|Dimensions|GetLength) 1))
    (if (Math|Conversions|ToBoolean(Integer) (Math|Integer|%(Integer) _index_3 (Variables|Measurements|GetDoor%20Counter)))
      (AddComponent|AddStaticMeshComponent false (Math|Transform|MakeTransform (Math|Vector|MakeVector _returnvalue_3 (Math|Conversions|ToFloat(Integer) (* _index_3 (Variables|Measurements|GetFloorSeparation))) 0.0) (Math|Rotator|MakeRotator 0.0 0.0 _returnvalue_4) "1.000000,1.000000,1.000000"))
      (else
        (AddComponent|AddStaticMeshComponent false (Math|Transform|MakeTransform (Math|Vector|MakeVector _returnvalue_3 (Math|Conversions|ToFloat(Integer) (* _index_3 (Variables|Measurements|GetFloorSeparation))) 0.0) (Math|Rotator|MakeRotator 0.0 0.0 _returnvalue_4) "1.000000,1.000000,1.000000")))))
  ;[0.15 0.15 0.15 0.5] Pared 2
  (for _index_4 (range 0 (- (Variables|Dimensions|GetWidth) 1))
    (AddComponent|AddStaticMeshComponent false (Math|Transform|MakeTransform (Math|Vector|MakeVector (Math|Conversions|ToFloat(Integer) (* _index_4 (Variables|Measurements|GetFloorSeparation))) (Math|Conversions|ToFloat(Integer) (* (Variables|Dimensions|GetLength) (Variables|Measurements|GetFloorSeparation))) 0.0) (Math|Rotator|MakeRotator 0.0 0.0 0.0) "1.000000,1.000000,1.000000")))
  ;[0.15 0.15 0.15 0.5] Pared 3
  (for _index_5 (range 0 (- (Variables|Dimensions|GetLength) 1))
    (AddComponent|AddStaticMeshComponent false (Math|Transform|MakeTransform (Math|Vector|MakeVector (Math|Conversions|ToFloat(Integer) (* 0 (Variables|Measurements|GetFloorSeparation))) (Math|Conversions|ToFloat(Integer) (* _index_5 (Variables|Measurements|GetFloorSeparation))) 0.0) (Math|Rotator|MakeRotator 0.0 0.0 (Math|Conversions|ToFloat(Integer) (- (Variables|Default|GetBaseRotation) 270))) "1.000000,1.000000,1.000000")))
  ;[0.15 0.15 0.15 0.5] Pared 4
  (for _index_6 (range 0 (- (Variables|Dimensions|GetWidth) 1))
    (AddComponent|AddStaticMeshComponent false (Math|Transform|MakeTransform (Math|Vector|MakeVector (Math|Conversions|ToFloat(Integer) (* _index_6 (Variables|Measurements|GetFloorSeparation))) (Math|Conversions|ToFloat(Integer) (* 0 (Variables|Measurements|GetFloorSeparation))) 0.0) (Math|Rotator|MakeRotator 0.0 0.0 0.0) "1.000000,1.000000,1.000000"))))